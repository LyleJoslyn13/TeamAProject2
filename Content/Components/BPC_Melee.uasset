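; BPC_Melee is a component that runs the player character's block and parry timing on the IA_Punch input.
; Starting a press off cooldown opens a brief parry window, sets the block duration and quarters walk speed.
; Tick counts down the cooldown and parry window, while holding the input drains block duration.
; Release, cancel or expiry passes through a shared DoOnce that starts the cooldown and restores saved speed.
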(event Input|EnhancedActionEvents|EnhancedInputActionIA_Punch
  (params (ActionValue :type Boolean) (ElapsedSeconds :type Float%20%28double-precision%29) (TriggeredSeconds :type Float%20%28double-precision%29) (InputAction :type Input%20Action%20Object%20Reference :default "/Game/FirstPerson/Input/Actions/IA_Punch.IA_Punch"))
  (bind _as_bp_lyles_fpscharacter (Variables|Default|GetAs%20BP%20Lyles%20FPSCharacter))
  (bind _charactermovement (Variables|/Script/Engine.Character|GetCharacterMovement _as_bp_lyles_fpscharacter))
  (bind _returnvalue (Class|MovementComponent|GetMaxSpeed _charactermovement))
  (:Triggered
    (if (<= (Variables|Default|GetBlockCD) 0.0)
      (Variables|Default|SetBlockDuration (- (Variables|Default|GetBlockDuration) (Utilities|Time|GetWorldDeltaSeconds)))
      (if (<= (Variables|Default|GetBlockDuration) 0.0)
        (Utilities|FlowControl|DoOnce false :!label _label
          (:Completed
            (Variables|Default|SetBlockCD 4.0)
            (Variables|Default|SetBlockDuration 2.5)
            (Variables|/Script/Engine.CharacterMovementComponent|SetMaxWalkSpeed (Variables|/Script/Engine.Character|GetCharacterMovement (Variables|Default|GetAs%20BP%20Lyles%20FPSCharacter)) (Variables|Default|GetBaseSpeed)))))))
  (:Started
    (if (<= (Variables|Default|GetBlockCD) 0.0)
      (Variables|Default|SetParryWindow 0.4)
      (Variables|Default|SetBlockDuration 2.5)
      (Variables|Default|SetBaseSpeed _returnvalue)
      (Variables|/Script/Engine.CharacterMovementComponent|SetMaxWalkSpeed _charactermovement (/ _returnvalue 4.0))
      (goto _label Reset)))
  (:Canceled
    (goto _label))
  (:Completed
    (goto _label)))

(event EventBeginPlay
  (bind _asbp_lyles_fpscharacter (Utilities|Casting|CastToBP_LylesFPSCharacter (Game|Player|GetPlayerPawn 0)))
  (Variables|Default|SetAs%20BP%20Lyles%20FPSCharacter _asbp_lyles_fpscharacter))

(event EventTick
  (params (DeltaSeconds :type Float%20%28single-precision%29))
  (Utilities|FlowControl|Sequence
    (:then_0
      (if (not (<= (Variables|Default|GetBlockCD) 0.0))
        (Variables|Default|SetBlockCD (- (Variables|Default|GetBlockCD) (Utilities|Time|GetWorldDeltaSeconds)))))
    (:then_1
      (if (> (Variables|Default|GetParryWindow) 0.0)
        (Variables|Default|SetParryWindow (- (Variables|Default|GetParryWindow) (Utilities|Time|GetWorldDeltaSeconds)))))))