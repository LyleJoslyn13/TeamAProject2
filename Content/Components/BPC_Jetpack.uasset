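; Player character component that adds a jetpack and limited air dashes through Enhanced Input.
; Pressing jump while falling zeroes gravity and sets upward velocity until release or the usage timer maxes out, after which the timer drains back down.
; Air dash launches along the last movement input with gravity off briefly; charges refill on ground contact polled after a normal jump.
; Timers and landing checks use DelayUntilNextTick loops instead of Tick.
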(event Custom|StopJetpack
  ;[1 1 1] Detecting if Jetpack should stop
  (CallFunction|DeActivateJetPack)
  (Character|StopJumping (Variables|Default|GetPlayerCharacter)))

(event Custom|DeActivateJetPack
  ;[1 1 1] Stop the Jet PAck
  (Variables|/Script/Engine.CharacterMovementComponent|SetGravityScale (Variables|/Script/Engine.Character|GetCharacterMovement (Variables|Default|GetPlayerCharacter)) 1.0)
  (bind _output_get (Variables|Default|SetisJetPackActive false))
  (if (not _output_get) :!label _label
    (if (> (Variables|Default|GetCurrentJetPackCooldown) 0.0)
      (Variables|Default|SetCurrentJetPackCooldown (- (Variables|Default|GetCurrentJetPackCooldown) (Utilities|Time|GetWorldDeltaSeconds)))
      (Utilities|FlowControl|DelayUntilNextTick)
      (goto _label)
      (else
        (Variables|Default|SetCurrentJetPackCooldown 0.0)))))

(event Custom|StartJetPack
  (bind _playercharacter (Variables|Default|GetPlayerCharacter))
  (bind _charactermovement (Variables|/Script/Engine.Character|GetCharacterMovement _playercharacter))
  ;[1 1 1] Start the Jetpack
  (Variables|/Script/Engine.CharacterMovementComponent|SetGravityScale _charactermovement 0.0)
  (Variables|/Script/Engine.MovementComponent|SetVelocity _charactermovement (Math|Vector|MakeVector (.x (Variables|/Script/Engine.MovementComponent|GetVelocity _charactermovement)) (.y (Variables|/Script/Engine.MovementComponent|GetVelocity _charactermovement)) (Variables|Default|GetJetpackVelocityZ)))
  (Variables|Default|SetisJetPackActive true))

(event Input|EnhancedActionEvents|EnhancedInputActionIA_AirDash
  (params (ActionValue :type Boolean) (ElapsedSeconds :type Float%20%28double-precision%29) (TriggeredSeconds :type Float%20%28double-precision%29) (InputAction :type Input%20Action%20Object%20Reference :default "/Game/FirstPerson/Input/Actions/IA_AirDash.IA_AirDash"))
  (bind _playercharacter (Variables|Default|GetPlayerCharacter))
  (bind _charactermovement (Variables|/Script/Engine.Character|GetCharacterMovement _playercharacter))
  ;[1 1 1] Air Dash
  (if (> (Variables|Default|GetCurrentAirDashes) 0)
    (if (not (Variables|Default|GetisAirDashing))
      (Variables|Default|SetisAirDashing true)
      (Variables|/Script/Engine.CharacterMovementComponent|SetGravityScale _charactermovement 0.0)
      (Character|LaunchCharacter _playercharacter (* (Class|Pawn|GetLastMovementInputVector _playercharacter) (Variables|Default|GetAirDashSpeed)) false false)
      (Utilities|FlowControl|Delay (Variables|Default|GetAirDashTime))
      (Variables|Default|SetisAirDashing false)
      (Variables|/Script/Engine.CharacterMovementComponent|SetGravityScale _charactermovement 1.0)
      (Math|Integer|DecrementInt (Variables|Default|GetCurrentAirDashes)))))

(event Input|EnhancedActionEvents|EnhancedInputActionIA_Jump
  (params (ActionValue :type Boolean) (ElapsedSeconds :type Float%20%28double-precision%29) (TriggeredSeconds :type Float%20%28double-precision%29) (InputAction :type Input%20Action%20Object%20Reference :default "/Game/FirstPerson/Input/Actions/IA_Jump.IA_Jump"))
  (bind _playercharacter (Variables|Default|GetPlayerCharacter))
  (bind _charactermovement (Variables|/Script/Engine.Character|GetCharacterMovement _playercharacter))
  (:Started
    ;[1 1 1] Detecting if Jumppack should start
    (if (AI|Components|NavMovement|IsFalling _charactermovement)
      (CallFunction|StartJetPack)
      (if (Variables|Default|GetisJetPackActive) :!label _label
        (bind _output_get (Variables|Default|SetCurrentJetPackCooldown (+ (Utilities|Time|GetWorldDeltaSeconds) (Variables|Default|GetCurrentJetPackCooldown))))
        (if (< _output_get (Variables|Default|GetMaxJetPackCooldown))
          (Utilities|FlowControl|DelayUntilNextTick)
          (goto _label)
          (else
            (CallFunction|StopJetpack))))
      (else
        (Character|Jump _playercharacter)
        (if (AI|Components|NavMovement|IsMovingonGround _charactermovement) :!label _label_2
          (Variables|Default|SetCurrentAirDashes (Variables|Default|GetMaxAirDashes))
          (else
            (Utilities|FlowControl|DelayUntilNextTick)
            (goto _label_2))))))
  (:Completed
    ;[1 1 1] Detecting if Jetpack should stop
    (if (Variables|Default|GetisJetPackActive)
      (CallFunction|DeActivateJetPack))
    (Character|StopJumping (Variables|Default|GetPlayerCharacter))))

(event EventBeginPlay)