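; BP_ExplosiveBullet is an expanding explosion area that damages enemies and then destroys itself.
; On BeginPlay, a DelayUntilNextTick loop, used in place of Tick, scales ExplosionRadius up or down between Scale and ScaleMultiplier over AnimationLength.
; Actors that begin overlapping ExplosionRadius take Damage only if their class exactly equals EnemyClass.
; Each overlap also prints a debug string.
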(event OnComponentBeginOverlap(ExplosionRadius)
  (params (OverlappedComponent :type Primitive%20Component%20Object%20Reference) (OtherActor :type Actor%20Object%20Reference) (OtherComp :type Primitive%20Component%20Object%20Reference) (OtherBodyIndex :type Integer) (bFromSweep :type Boolean) (SweepResult :type Hit%20Result%20Structure%20%28by%20ref%29))
  (Development|PrintString "overlap")
  (if (== (Utilities|GetClass OtherActor) (Variables|Default|GetEnemyClass))
    (Game|Damage|ApplyDamage OtherActor (Variables|Default|GetDamage) 0 0)))

(event EventBeginPlay
  (Transformation|SetRelativeScale3D (Variables|Default|GetExplosionRadius) (Math|Vector|MakeVector (Math|Float|MapRangeClamped (Variables|Default|GetAnimationTIme) 0.0 (Variables|Default|GetAnimationLength) (Variables|Default|GetScale) (Variables|Default|GetScaleMultiplier)) (Math|Float|MapRangeClamped (Variables|Default|GetAnimationTIme) 0.0 (Variables|Default|GetAnimationLength) (Variables|Default|GetScale) (Variables|Default|GetScaleMultiplier)) (Math|Float|MapRangeClamped (Variables|Default|GetAnimationTIme) 0.0 (Variables|Default|GetAnimationLength) (Variables|Default|GetScale) (Variables|Default|GetScaleMultiplier))) :!label _label)
  (if (>= (Variables|Default|GetAnimationTIme) (Variables|Default|GetAnimationLength))
    (Actor|DestroyActor)
    (else
      (Variables|Default|SetAnimationTIme (+ (Variables|Default|GetAnimationTIme) (Utilities|Time|GetWorldDeltaSeconds)))
      (Utilities|FlowControl|DelayUntilNextTick)
      (goto _label))))

(event Collision|EventActorBeginOverlap
  (params (OtherActor :type Actor%20Object%20Reference)))

(event EventTick
  (params (DeltaSeconds :type Float%20%28single-precision%29)))

(fn ConstructionScript)