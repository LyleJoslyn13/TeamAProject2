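; BP_Explosive is a timed explosive actor that detonates on its own roughly two seconds after BeginPlay, with slightly randomized timing.
; Detonation resizes the ExplosionRadius sphere with an overlap update, spawns a Niagara effect at the Cube, and hides the Cube.
; The explosion sound plays at world origin, not at the actor.
; The actor destroys itself after a short delay and contains no damage or overlap-response logic.
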(event EventBeginPlay
  (Utilities|FlowControl|Delay (Math|Random|RandomFloatinRange 1.9 2.1))
  (Components|Sphere|SetSphereRadius (Variables|Default|GetexplosionRadius) 1e+02 true)
  (Niagara|SpawnSystematLocation "/Game/Particles/NS_Explosion.NS_Explosion" (Transformation|GetWorldLocation (Variables|Default|GetCube)) "0, 0, 0" "0.900000,0.900000,0.900000")
  (Audio|PlaySoundatLocation "/Game/SFX/51467__smcameron__missile_explosion.51467__smcameron__missile_explosion" "0, 0, 0" "0, 0, 0" 0.1 1.0 0.0 0 0 0 0)
  (Rendering|SetVisibility (Variables|Default|GetCube) false false)
  (Utilities|FlowControl|Delay 0.5)
  (Actor|DestroyActor))

(fn ConstructionScript)