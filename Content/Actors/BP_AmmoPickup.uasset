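; BP_AmmoPickup is a pickup actor that adds reserve sniper ammo when the player character overlaps it.
; Its Collision overlap event checks for the first player's character, casts it to BP_LylesFPSCharacter and caches the reference.
; A switch on AmmoType then increases the matching Explosive, Laser or Railgun reserve on the character's BPCSniper component.
; The graph never destroys or disables the actor, so each new overlap grants ammo again.
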(event OnComponentBeginOverlap(Collision)
  (params (OverlappedComponent :type Primitive%20Component%20Object%20Reference) (OtherActor :type Actor%20Object%20Reference) (OtherComp :type Primitive%20Component%20Object%20Reference) (OtherBodyIndex :type Integer) (bFromSweep :type Boolean) (SweepResult :type Hit%20Result%20Structure%20%28by%20ref%29))
  (if (== OtherActor (Game|GetPlayerCharacter 0))
    (bind _asbp_lyles_fpscharacter (Utilities|Casting|CastToBP_LylesFPSCharacter OtherActor))
    (bind _output_get (Variables|Default|SetPlayerCharacter _asbp_lyles_fpscharacter))
    (switch Utilities|FlowControl|Switch|SwitchonE_AmmoTypes (Variables|Default|GetAmmoType)
      (:NewEnumerator1
        (Variables|/Game/Components/SniperSystem/BPC_Sniper.BPC_Sniper_C|SetReserveExplosiveAmmo (Variables|/Game/FirstPerson/Blueprints/BP_LylesFPSCharacter.BP_LylesFPSCharacter_C|GetBPC_Sniper _output_get) (+ (Variables|/Game/Components/SniperSystem/BPC_Sniper.BPC_Sniper_C|GetReserveExplosiveAmmo (Variables|/Game/FirstPerson/Blueprints/BP_LylesFPSCharacter.BP_LylesFPSCharacter_C|GetBPC_Sniper _output_get)) 5.0)))
      (:NewEnumerator2
        (Math|Float|IncrementFloat (Variables|/Game/Components/SniperSystem/BPC_Sniper.BPC_Sniper_C|GetReserveLaserAmmo (Variables|/Game/FirstPerson/Blueprints/BP_LylesFPSCharacter.BP_LylesFPSCharacter_C|GetBPC_Sniper _output_get))))
      (:NewEnumerator3
        (Math|Float|IncrementFloat (Variables|/Game/Components/SniperSystem/BPC_Sniper.BPC_Sniper_C|GetReserveRailGunAmmo (Variables|/Game/FirstPerson/Blueprints/BP_LylesFPSCharacter.BP_LylesFPSCharacter_C|GetBPC_Sniper _output_get)))))))

(event EventBeginPlay)

(event Collision|EventActorBeginOverlap
  (params (OtherActor :type Actor%20Object%20Reference)))

(event EventTick
  (params (DeltaSeconds :type Float%20%28single-precision%29)))

(fn ConstructionScript)