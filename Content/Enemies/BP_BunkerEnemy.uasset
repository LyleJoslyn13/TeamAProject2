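; Bunker enemy that chases a seen player and is only damageable while exposed, shown by swapping its body mesh.
; Within close range it becomes an invulnerable Cube; farther away, a DoOnce switches it to a vulnerable Cone.
; It turns toward the player and uses AIMoveTo; on arrival, if off cooldown, it opens up and box-traces forward.
; After a delay it closes again and damages the player if hit.
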(event OnSeePawn(PawnSensing)
  (params (Pawn :type Pawn%20Object%20Reference))
  (bind _returnvalue (Transformation|GetActorLocation))
  (bind _body (Variables|Default|Getbody))
  (bind _returnvalue_2 (Transformation|GetWorldLocation _body))
  (bind _asbp_lyles_fpscharacter (Utilities|Casting|CastToBP_LylesFPSCharacter Pawn))
  (Variables|Default|SetPlayer _asbp_lyles_fpscharacter)
  (if (<= (Math|Vector|Distance(Vector) _returnvalue (Transformation|GetActorLocation (Variables|Default|GetPlayer))) 1.5e+03)
    (Components|StaticMesh|SetStaticMesh (Variables|Default|Getbody) "/Engine/BasicShapes/Cube.Cube")
    (Variables|Default|SetCanTakeDamage false)
    (Utilities|FlowControl|Sequence
      (:then_0
        (goto _label_2 Reset))
      (:then_1
        (Transformation|SetWorldRotation (Variables|Default|Getbody) (Math|Rotator|MakeRotator 0.0 0.0 (.yaw (Math|Interpolation|RInterpTo (Transformation|GetActorRotation) (Math|Rotator|FindLookatRotation _returnvalue (Transformation|GetActorLocation (Variables|Default|GetPlayer))) (Utilities|Time|GetWorldDeltaSeconds) 1e+02))) false false :!label _label)
        (AI|AIMoveTo self (Math|Vector|MakeVector (.x (Transformation|GetActorLocation (Variables|Default|GetPlayer))) (.y (Transformation|GetActorLocation (Variables|Default|GetPlayer))) (.z (Transformation|GetActorLocation (Variables|Default|GetPlayer)))) 0 2e+02 false
          (:OnSuccess
            (if (<= (Variables|Default|GetattackCD) 0.0)
              (Utilities|FlowControl|Delay 0.5)
              (Components|StaticMesh|SetStaticMesh (Variables|Default|Getbody) "/Engine/BasicShapes/Cone.Cone")
              (Variables|Default|SetCanTakeDamage true)
              (bind _outhit (Collision|BoxTraceByChannel _returnvalue_2 (+ _returnvalue_2 (* (Math|Vector|GetForwardVector _body) (Variables|Default|Getrange))) "0.000000,50.000000,20.000000" (Transformation|GetWorldRotation _body) "TraceTypeQuery1" false 0 "ForDuration" true "(R=1.000000,G=0.000000,B=0.000000,A=1.000000)" "(R=0.000000,G=1.000000,B=0.000000,A=1.000000)" 2.0))
              (Variables|Default|SetattackCD 3.0)
              (Utilities|FlowControl|Delay 2.0)
              (Components|StaticMesh|SetStaticMesh (Variables|Default|Getbody) "/Engine/BasicShapes/Cube.Cube")
              (Variables|Default|SetCanTakeDamage false)
              (if (== (Utilities|GetClass (.HitActor (Collision|BreakHitResult _outhit))) (Variables|Default|GetPlayer%20Class))
                (Game|Damage|ApplyDamage (.HitActor (Collision|BreakHitResult _outhit)) 15.0 0 0)))))))
    (else
      (Utilities|FlowControl|Sequence
        (:then_0
          (goto _label))
        (:then_1
          (Utilities|FlowControl|DoOnce false :!label _label_2
            (:Completed
              (Components|StaticMesh|SetStaticMesh (Variables|Default|Getbody) "/Engine/BasicShapes/Cone.Cone")
              (Variables|Default|SetCanTakeDamage true))))))))

(event EventBeginPlay
  (Variables|Default|SetPlayer%20Class "/Game/FirstPerson/Blueprints/BP_LylesFPSCharacter.BP_LylesFPSCharacter_C"))

(event EventTick
  (params (DeltaSeconds :type Float%20%28single-precision%29))
  (if (>= (Variables|Default|GetattackCD) 0.0)
    (Variables|Default|SetattackCD (- (Variables|Default|GetattackCD) (Utilities|Time|GetWorldDeltaSeconds)))))

(event Game|Damage|EventAnyDamage
  (params (Damage :type Float%20%28single-precision%29) (DamageType :type Damage%20Type%20Object%20Reference) (InstigatedBy :type Controller%20Object%20Reference) (DamageCauser :type Actor%20Object%20Reference))
  (if (Variables|Default|GetCanTakeDamage)
    (bind _output_get (Variables|Default|SetCurrent%20Health (- (Variables|Default|GetCurrent%20Health) Damage)))
    (if (<= _output_get 0.0)
      (Actor|DestroyActor))))

(fn ConstructionScript)