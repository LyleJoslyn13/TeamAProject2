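; BP_ExplosiveEnemy is a suicide enemy that chases the player on sight and explodes when close or when its health runs out.
; PawnSensing drives an AI move toward the seen player's position, and arrival or lethal damage calls Explode.
; Explode stops new chases, swaps the body material as a delayed fuse, then enlarges a sphere whose begin-overlap damages the player.
; Niagara and sound effects accompany the blast before the actor destroys itself.
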(event OnSeePawn(PawnSensing)
  (params (Pawn :type Pawn%20Object%20Reference))
  (if (Variables|Default|GetcanMove)
    (bind _asbp_lyles_fpscharacter (Utilities|Casting|CastToBP_LylesFPSCharacter Pawn))
    (AI|AIMoveTo self (Math|Vector|MakeVector (.x (Transformation|GetActorLocation _asbp_lyles_fpscharacter)) (.y (Transformation|GetActorLocation _asbp_lyles_fpscharacter)) 1e+02) 0 2e+02 false
      (:OnSuccess
        (CallFunction|Explode)))))

(event OnComponentBeginOverlap(ExplosionRadius)
  (params (OverlappedComponent :type Primitive%20Component%20Object%20Reference) (OtherActor :type Actor%20Object%20Reference) (OtherComp :type Primitive%20Component%20Object%20Reference) (OtherBodyIndex :type Integer) (bFromSweep :type Boolean) (SweepResult :type Hit%20Result%20Structure%20%28by%20ref%29))
  (if (== (Utilities|GetClass OtherActor) (Variables|Default|GetPlayer%20Class))
    (Game|Damage|ApplyDamage OtherActor 2e+01 0 0)))

(event Custom|Explode
  (Variables|Default|SetcanMove false)
  (Rendering|Material|SetMaterial (Variables|Default|Getbody) 0 "/Engine/MapTemplates/Materials/BasicAsset01.BasicAsset01")
  (Utilities|FlowControl|Delay 2.0)
  (Components|Sphere|SetSphereRadius (Variables|Default|GetExplosionRadius) 2.5e+02 true)
  (Niagara|SpawnSystematLocation "/Game/Particles/NS_Explosion.NS_Explosion" (Transformation|GetWorldLocation (Variables|Default|Getbody)) "0, 0, 0" "2.500000,2.500000,2.500000")
  (Audio|PlaySoundatLocation "/Game/SFX/51467__smcameron__missile_explosion.51467__smcameron__missile_explosion" "0, 0, 0" "0, 0, 0" 1.0 1.0 0.0 0 0 0 0)
  (Rendering|SetVisibility (Variables|Default|Getbody) false false)
  (Utilities|FlowControl|Delay 0.5)
  (Actor|DestroyActor))

(event EventBeginPlay
  (Variables|Default|SetPlayer%20Class "/Game/FirstPerson/Blueprints/BP_LylesFPSCharacter.BP_LylesFPSCharacter_C"))

(event Game|Damage|EventAnyDamage
  (params (Damage :type Float%20%28single-precision%29) (DamageType :type Damage%20Type%20Object%20Reference) (InstigatedBy :type Controller%20Object%20Reference) (DamageCauser :type Actor%20Object%20Reference))
  (bind _output_get (Variables|Default|SetCurrent%20Health (- (Variables|Default|GetCurrent%20Health) Damage)))
  (if (<= _output_get 0.0)
    (CallFunction|Explode)))

(fn ConstructionScript)